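; BP_BlockSpawner tracks the blocks in the level and signals a win when none remain; despite its name, it spawns nothing.
; On BeginPlay it counts all BP_Block actors, binds to each one's OnBlockDead event and caches the BP_Plate.
; Change Score forwards points to the plate, decrements the remaining count, then fires either the WinGame or BlockDead dispatcher.
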(event EventBeginPlay
  (Utilities|FlowControl|Sequence
    (:then_0
      (bind _outactors (Actor|GetAllActorsOfClass "/Game/Actors/BP_Block.BP_Block_C"))
      (bind _output_get (Variables|Default|SetAmountBlocks _outactors))
      (Variables|Default|SetBlocksLeft (Utilities|Array|Length _output_get))
      (for _array_element _output_get
        (EventDispatchers|BindEventtoOnBlockDead _array_element (EventDispatchers|CreateEvent :!event ChangeScore))))
    (:then_1
      (bind _returnvalue (Actor|GetActorOfClass "/Game/Actors/BP_Plate.BP_Plate_C"))
      (Variables|Default|SetPawn _returnvalue))))

(event Collision|EventActorBeginOverlap
  (params (OtherActor :type Actor%20Object%20Reference)))

(event EventTick
  (params (DeltaSeconds :type Float%20%28single-precision%29)))

(fn ConstructionScript)

(fn ChangeScore
  (params (Score :type Integer) (BlocksLeft :type Integer))
  (Default|ChangeScore (Variables|Default|GetPawn) Score)
  (bind _output_get (Variables|Default|SetBlocksLeft (- (Variables|Default|GetBlocksLeft) 1)))
  (if (== _output_get 0)
    (Default|CallWinGame)
    (else
      (Default|CallBlockDead _output_get))))