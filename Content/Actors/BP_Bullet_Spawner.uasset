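; BP_Bullet_Spawner is a short-lived actor that gives BP_Plate a temporary twin-gun firing burst.
; On BeginPlay, a DoN loop with a delay shows the plate's Gun1 and Gun2 components and spawns a BP_Bullet at each, once per second for seven volleys.
; A parallel sequence branch waits just past the final volley, hides both guns and destroys the spawner.
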(event EventBeginPlay
  (Utilities|FlowControl|Sequence
    (:then_0
      (Utilities|FlowControl|DoN 7 :!label _label
        (:Exit
          (Utilities|FlowControl|Delay 1.0)
          (bind _returnvalue (Actor|GetActorOfClass "/Game/Actors/BP_Plate.BP_Plate_C"))
          (Rendering|SetVisibility (Variables|/Game/Actors/BP_Plate.BP_Plate_C|GetGun1 _returnvalue) true false)
          (Game|SpawnActorfromClass "/Game/Actors/BP_Bullet.BP_Bullet_C" (Math|Transform|MakeTransform (Transformation|GetWorldLocation (Variables|/Game/Actors/BP_Plate.BP_Plate_C|GetGun1 _returnvalue)) "0, 0, 0" "1.000000,1.000000,1.000000") "AlwaysSpawn" "MultiplyWithRoot" 0 0)
          (Game|SpawnActorfromClass "/Game/Actors/BP_Bullet.BP_Bullet_C" (Math|Transform|MakeTransform (Transformation|GetWorldLocation (Variables|/Game/Actors/BP_Plate.BP_Plate_C|GetGun2 _returnvalue)) "0, 0, 0" "1.000000,1.000000,1.000000") "AlwaysSpawn" "MultiplyWithRoot" 0 0)
          (goto _label))))
    (:then_1
      (Utilities|FlowControl|Delay 8.1)
      (Actor|GetActorOfClass "/Game/Actors/BP_Plate.BP_Plate_C")
      (Rendering|SetVisibility (Variables|/Game/Actors/BP_Plate.BP_Plate_C|GetGun1 _returnvalue) false false)
      (Actor|DestroyActor))))

(event Collision|EventActorBeginOverlap
  (params (OtherActor :type Actor%20Object%20Reference)))

(event EventTick
  (params (DeltaSeconds :type Float%20%28single-precision%29)))

(fn ConstructionScript)