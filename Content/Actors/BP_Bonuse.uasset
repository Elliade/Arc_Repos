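; BP_Bonuse is a moving bonus pickup actor with eight random types, such as pawn size, ball speed, health change, guns, bomb and extra ball.
; The construction script rolls BonusType, adds a static mesh for it and sets Score for some types.
; Tick shifts it along +Y by a fixed, frame-rate-dependent step, and overlapping a KillZVolume destroys it.
; The file itself applies no bonus effects.
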(event EventBeginPlay)

(event Collision|EventActorBeginOverlap
  (params (OtherActor :type Actor%20Object%20Reference))
  ;[1 1 1] Удаление бонуса
  (Utilities|Casting|CastToKillZVolume OtherActor)
  (Actor|DestroyActor))

(event EventTick
  (params (DeltaSeconds :type Float%20%28single-precision%29))
  ;[1 1 1] Движение бонуса
  (Transformation|AddWorldOffset (Variables|Default|GetDefaultSceneRoot) "0.000000,10.000000,0.000000" false false))

(fn ConstructionScript
  (bind _output_get (Variables|Default|SetBonus_Type (Math|Random|RandomIntegerinRange 1 8)))
  (switch int _output_get
    (:1
      ;[1 1 1] Размер пешки
      (AddComponent|AddStaticMeshComponent false)
      (Variables|Default|SetScore 5))
    (:2
      ;[1 1 1] Скорость мячика
      (AddComponent|AddStaticMeshComponent false)
      (Variables|Default|SetScore 5))
    (:3
      ;[1 1 1] Увеличение ХП пешки
      (AddComponent|AddStaticMeshComponent false))
    (:4
      ;[1 1 1] Уменьшение ХП пешки
      (AddComponent|AddStaticMeshComponent false)
      (Variables|Default|SetScore -15))
    (:5
      ;[1 1 1] Пушки
      (AddComponent|AddStaticMeshComponent false))
    (:6
      ;[1 1 1] Добавить очки
      (AddComponent|AddStaticMeshComponent false)
      (Variables|Default|SetScore 100))
    (:7
      ;[1 1 1] Бомба
      (AddComponent|AddStaticMeshComponent false))
    (:8
      ;[1 1 1] Бонусный мяч
      (AddComponent|AddStaticMeshComponent false)
      (Variables|Default|SetScore 5))))