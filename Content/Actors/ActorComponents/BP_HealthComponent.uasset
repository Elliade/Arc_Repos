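; BP_HealthComponent is an actor component that tracks an HP value and reports health changes and death through event calls.
; Add and Sub step HP by one and pass the result to Update, with no clamping.
; Update fires OnHealthUpdate with old and new health, stores HP, then fires OnDeath when the Death check finds HP at or below zero.
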(event EventBeginPlay)

(event EventTick
  (params (DeltaSeconds :type Float%20%28single-precision%29)))

(fn Update
  (params (HP :type Integer))
  (Default|CallOnHealthUpdate (Variables|Default|GetHP) HP)
  (Variables|Default|SetHP HP)
  (if (CallFunction|Death)
    (Default|CallOnDeath)))

(fn Sub
  (CallFunction|Update (- (Variables|Default|GetHP) 1)))

(fn Add
  (CallFunction|Update (+ (Variables|Default|GetHP) 1)))

(fn Death
  (return (<= (Variables|Default|GetHP) 0)))