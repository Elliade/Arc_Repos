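; BP_Block is a breakable block with random 1–3 HP, color-coded by health, that scores more the lower its starting HP.
; The construction script rolls HP, sets material and score, and binds health component events.
; Ball or bonus-ball hits and bullet overlaps subtract health; material updates as it drops.
; DestroyBlock broadcasts the score, destroys the actor and spawns a bonus pickup, currently weighted at 100%.
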(event EventBeginPlay)

(event EventTick
  (params (DeltaSeconds :type Float%20%28single-precision%29)))

(event Collision|EventHit
  (params (MyComp :type Primitive%20Component%20Object%20Reference) (Other :type Actor%20Object%20Reference) (OtherComp :type Primitive%20Component%20Object%20Reference) (bSelfMoved :type Boolean) (HitLocation :type Vector :default "0, 0, 0") (HitNormal :type Vector :default "0, 0, 0") (NormalImpulse :type Vector :default "0, 0, 0") (Hit :type Hit%20Result%20Structure%20%28by%20ref%29))
  ;[1 1 1] Взаимодействие с мячиками
  (Utilities|Casting|CastToBP_Ball Other
    (:then
      _)
    (:CastFailed
      (Utilities|Casting|CastToBP_BonuseBall Other)))
  (Default|Sub (Variables|Default|GetBP_HealthComponent)))

(event Collision|EventActorBeginOverlap
  (params (OtherActor :type Actor%20Object%20Reference))
  (Utilities|Casting|CastToBP_Bullet OtherActor)
  ;[1 1 1] Взаимодействие с мячиками
  (Default|Sub (Variables|Default|GetBP_HealthComponent)))

(fn ConstructionScript
  (bind _bp_healthcomponent (Variables|Default|GetBP_HealthComponent))
  (bind _cube (Variables|Default|GetCube))
  ;[1 1 1] ХП и цвет блоков
  (Variables|/Game/Actors/ActorComponents/BP_HealthComponent.BP_HealthComponent_C|SetHP _bp_healthcomponent (Math|Random|RandomIntegerinRange 1 3))
  (CallFunction|Binds)
  (if (== (Variables|/Game/Actors/ActorComponents/BP_HealthComponent.BP_HealthComponent_C|GetHP _bp_healthcomponent) 3)
    (Rendering|Material|SetMaterial _cube 0 "/Game/Actors/Materials/Textures/Red.Red")
    (Variables|Default|SetScore 1)
    (elif (== (Variables|/Game/Actors/ActorComponents/BP_HealthComponent.BP_HealthComponent_C|GetHP _bp_healthcomponent) 2)
      (Rendering|Material|SetMaterial _cube 0 "/Game/Actors/Materials/Textures/Yellow.Yellow")
      (Variables|Default|SetScore 3)
      (else
        (Rendering|Material|SetMaterial _cube 0 "/Game/Actors/Materials/Textures/Green.Green")
        (Variables|Default|SetScore 7)))))

(fn Binds
  (bind _bp_healthcomponent (Variables|Default|GetBP_HealthComponent))
  (EventDispatchers|BindEventtoOnHealthUpdate _bp_healthcomponent (EventDispatchers|CreateEvent :!event SetMaterial))
  (EventDispatchers|BindEventtoOnDeath _bp_healthcomponent (EventDispatchers|CreateEvent :!event DestroyBlock)))

(fn SetMaterial
  (params (OldHealth :type Integer) (NewHealth :type Integer))
  (bind _cube (Variables|Default|GetCube))
  ;[1 1 1] Изменение материала при ударе
  (if (== NewHealth 2)
    (Rendering|Material|SetMaterial _cube 0 "/Game/Actors/Materials/Textures/Yellow.Yellow")
    (elif (== NewHealth 1)
      (Rendering|Material|SetMaterial _cube 0 "/Game/Actors/Materials/Textures/Green.Green"))))

(fn DestroyBlock
  ;[1 1 1] Спавн бонуса
  (Default|CallOnBlockDead (Variables|Default|GetScore))
  (Actor|DestroyActor)
  (if (Math|Random|RandomBoolwithWeight 1.0)
    (Game|SpawnActorfromClass "/Game/Actors/BP_Bonuse.BP_Bonuse_C" (Math|Transform|MakeTransform (.location (Transformation|GetActorTransform)) "180.000000,0.000000,90.000000" "1.000000,1.000000,1.000000") "AlwaysSpawn" "MultiplyWithRoot" 0 0)))