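; BP_Plate is the player paddle in a brick-breaker game, moved sideways by axis input with swept offsets and directional spotlights.
; It spawns the ball and HUD, tracks score, and binds health and ball-death delegates for respawning and game flow.
; Overlapped bonuses dispatch by type to paddle, ball, health, bullet or bomb effects, with retriggerable delays undoing size and speed changes.
; Win and loss functions swap the HUD for a result screen.
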(event Custom|Size%20Time
  ;[1 1 1] Вертаем взад исходный размер пешки
  (Utilities|FlowControl|RetriggerableDelay 1e+01)
  (Transformation|SetRelativeScale3D (Variables|Default|GetPlate) (Variables|Default|GetBaseScale)))

(event Custom|Speed%20Time
  ;[1 1 1] Вертаем взад исходную скорость мячика
  (Utilities|FlowControl|RetriggerableDelay 5.0)
  (bind _returnvalue (Actor|GetActorOfClass "/Game/Actors/BP_Ball.BP_Ball_C"))
  (Variables|/Game/Actors/BP_Ball.BP_Ball_C|SetVelocity _returnvalue (Variables|/Game/Actors/BP_Ball.BP_Ball_C|GetBase_Velocity _returnvalue)))

(event Custom|Win%20Game)

(event EventBeginPlay
  (bind _returnvalue (Game|GetPlayerCameraManager 0))
  (bind _returnvalue_2 (Game|Player|GetOwningPlayerController _returnvalue))
  ;[1 1 1] Старт игры
  (Variables|Default|SetBaseScale (Variables|/Script/Engine.SceneComponent|GetRelativeScale3D (Variables|Default|GetPlate)))
  (Utilities|FlowControl|Sequence
    (:then_0
      (bind _returnvalue_3 (Actor|GetActorOfClass "/Game/Actors/BP_BlockSpawner.BP_BlockSpawner_C"))
      (EventDispatchers|BindEventtoWinGame _returnvalue_3 (delegate Custom|Win%20Game)))
    (:then_1
      (CallFunction|Binds)
      (CallFunction|SpawnBall)
      (Input|SetInputModeGameOnly _returnvalue_2 false)
      (bind _returnvalue_4 (UserInterface|CreateWidget "/Game/UI/WBP_HUD.WBP_HUD_C" _returnvalue_2))
      (UserInterface|Viewport|AddtoViewport _returnvalue_4 0)
      (Variables|Default|SetHUD _returnvalue_4))))

(event Collision|EventActorBeginOverlap
  (params (OtherActor :type Actor%20Object%20Reference))
  ;[1 1 1] Ловим бонус
  (bind _asbp_bonuse (Utilities|Casting|CastToBP_Bonuse OtherActor))
  (Variables|Default|SetGameScore (+ (Variables|/Game/Actors/BP_Bonuse.BP_Bonuse_C|GetScore _asbp_bonuse) (Variables|Default|GetGameScore)))
  (CallFunction|BonuseChooseEffects 0 (Variables|/Game/Actors/BP_Bonuse.BP_Bonuse_C|GetBonus_Type _asbp_bonuse)))

(event Input|AxisEvents|InputAxisMovement
  (params (AxisValue :type Float%20%28single-precision%29))
  (bind _spotlight (Variables|Default|GetSpotLight))
  ;[1 1 1] Движение пешки
  (if (> AxisValue 0.0)
    (Transformation|AddActorWorldOffset "-50.000000,0.000000,0.000000" true)
    (Rendering|SetVisibility _spotlight true false)
    (else
      (Rendering|SetVisibility _spotlight false false))))

(event Input|AxisEvents|InputAxisMovement
  (params (AxisValue :type Float%20%28single-precision%29))
  (bind _spotlight1 (Variables|Default|GetSpotLight1))
  ;[1 1 1] Движение пешки
  (if (< AxisValue 0.0)
    (Transformation|AddActorWorldOffset "50.000000,0.000000,0.000000" true)
    (Rendering|SetVisibility _spotlight1 true false)
    (else
      (Rendering|SetVisibility _spotlight1 false false))))

(fn ConstructionScript)

(fn Binds
  (bind _bp_healthcomponent (Variables|Default|GetBP_HealthComponent))
  (EventDispatchers|BindEventtoOnHealthUpdate _bp_healthcomponent (EventDispatchers|CreateEvent :!event HPUpdate))
  (EventDispatchers|BindEventtoOnDeath _bp_healthcomponent (EventDispatchers|CreateEvent :!event GameEnd)))

(fn SpawnBall
  ;[1 1 1] Спавн основного мячика
  (bind _returnvalue (Game|SpawnActorfromClass "/Game/Actors/BP_Ball.BP_Ball_C" (Math|Transform|MakeTransform (Transformation|GetWorldLocation (Variables|Default|GetSphere)) "0, 0, 0" "1.000000,1.000000,1.000000") "AlwaysSpawn" "MultiplyWithRoot" 0 0))
  (bind _output_get (Variables|Default|SetBP_Ball _returnvalue))
  (EventDispatchers|BindEventtoOnDead _output_get (EventDispatchers|CreateEvent :!event RespawnBall))
  (return))

(fn RespawnBall
  ;[1 1 1] Респавн основного мячика
  (Default|Sub (Variables|Default|GetBP_HealthComponent))
  (CallFunction|SpawnBall))

(fn GameWin
  (bind _returnvalue (Game|GetPlayerCameraManager 0))
  (bind _returnvalue_2 (Game|Player|GetOwningPlayerController _returnvalue))
  (Widget|SetVisibility (Variables|Default|GetHUD) "Collapsed")
  (bind _returnvalue_3 (UserInterface|CreateWidget "/Game/UI/WBP_WinScreen.WBP_WinScreen_C" _returnvalue_2))
  (Default|UpdateWinner _returnvalue_3 true)
  (UserInterface|Viewport|AddtoViewport _returnvalue_3 0)
  (Input|SetInputModeUIOnly 0 _returnvalue_3 "LockOnCapture" false)
  (Variables|/Script/Engine.PlayerController|SetbShowMouseCursor _returnvalue_2 true)
  (AddComponent|AddAudioComponent false))

(fn GameEnd
  (bind _returnvalue (Game|GetPlayerCameraManager 0))
  (bind _returnvalue_2 (Game|Player|GetOwningPlayerController _returnvalue))
  (Default|CallGameEnd)
  (Widget|SetVisibility (Variables|Default|GetHUD) "Collapsed")
  (bind _returnvalue_3 (UserInterface|CreateWidget "/Game/UI/WBP_WinScreen.WBP_WinScreen_C" _returnvalue_2))
  (Default|UpdateWinner _returnvalue_3 false)
  (UserInterface|Viewport|AddtoViewport _returnvalue_3 0)
  (Input|SetInputModeUIOnly 0 _returnvalue_3 "LockOnCapture" false)
  (Variables|/Script/Engine.PlayerController|SetbShowMouseCursor _returnvalue_2 true)
  (AddComponent|AddAudioComponent false))

(fn HPUpdate
  (params (OldHealth :type Integer) (NewHealth :type Integer))
  (Variables|Default|SetHP (Variables|/Game/Actors/ActorComponents/BP_HealthComponent.BP_HealthComponent_C|GetHP (Variables|Default|GetBP_HealthComponent))))

(fn ChangeScore
  (params (Amount :type Integer))
  (bind _output_get (Variables|Default|SetGameScore (+ Amount (Variables|Default|GetGameScore))))
  (Default|CallOnScoreChange _output_get))

(fn BonuseChooseEffects
  (params (BonuseScore :type Integer) (Bonuse_Type :type Integer))
  (switch int Bonuse_Type
    (:1
      (CallFunction|BonuseDescreasePawnScale)
      (Audio|PlaySound2D "/Game/Sounds/SC_D_Bonuse.SC_D_Bonuse" 1.0 1.0 0.0 0 0 :!label _label))
    (:2
      (CallFunction|BonuseAddBallSpeed)
      (Audio|PlaySound2D "/Game/Sounds/SC_Up_Bonuse.SC_Up_Bonuse" 1.0 1.0 0.0 0 0 :!label _label_2))
    (:3
      (CallFunction|BonuseAddHP)
      (goto _label_2))
    (:4
      (CallFunction|BonuseSubHP)
      (goto _label))
    (:5
      (CallFunction|BonuseGuns)
      (goto _label_2))
    (:6
      (CallFunction|BonuseScore)
      (goto _label_2))
    (:7
      (CallFunction|BonuseBomb)
      (goto _label))
    (:8
      (CallFunction|BonuseSpawnBonuseBall)
      (goto _label_2)))
  (return))

(fn BonuseDescreasePawnScale
  (params (Object :type Object%20Object%20Reference))
  (bind _plate (Variables|Default|GetPlate))
  (bind _relativescale3d (Variables|/Script/Engine.SceneComponent|GetRelativeScale3D _plate))
  ;[1 1 1] Уменьшаем размер пешки
  (Transformation|SetRelativeScale3D (Variables|Default|GetPlate) (Math|Vector|MakeVector (* (.x _relativescale3d) 0.7) (.y _relativescale3d) (.z _relativescale3d)))
  (CallFunction|SizeTime))

(fn BonuseAddBallSpeed
  (bind _returnvalue (Actor|GetActorOfClass "/Game/Actors/BP_Ball.BP_Ball_C"))
  (Variables|/Game/Actors/BP_Ball.BP_Ball_C|SetVelocity _returnvalue (+ (Variables|/Game/Actors/BP_Ball.BP_Ball_C|GetVelocity _returnvalue) 15.0))
  (CallFunction|SpeedTime))

(fn BonuseAddHP
  (Default|Add (Variables|Default|GetBP_HealthComponent))
  (return))

(fn BonuseSubHP
  (Default|Sub (Variables|Default|GetBP_HealthComponent))
  (return))

(fn BonuseGuns
  (Game|SpawnActorfromClass "/Game/Actors/BP_Bullet.BP_Bullet_C" (Math|Conversions|ToTransform(Vector) (Transformation|GetWorldLocation (Variables|Default|GetSphere))) "Undefined" "MultiplyWithRoot" 0 0)
  (return))

(fn BonuseScore)

(fn BonuseBomb
  (Default|CallOnDeath (Variables|Default|GetBP_HealthComponent))
  (return))

(fn BonuseSpawnBonuseBall
  ;[1 1 1] Спавн бонусного мячика
  (Game|SpawnActorfromClass "/Game/Actors/BP_BonuseBall.BP_BonuseBall_C" (Math|Transform|MakeTransform (Transformation|GetWorldLocation (Variables|Default|GetSphere)) "0, 0, 0" "1.000000,1.000000,1.000000") "AlwaysSpawn" "MultiplyWithRoot" 0 0)
  (return))

(fn WinGame)